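; BP_DestructibleActor is an explosive destructible that loses Life from any damage and can set off a blast at zero.
; At zero or below, a debug-drawn multi-sphere trace on the Visibility channel finds nearby hits and applies fixed damage to each hit actor.
; The explosion Niagara spawn and DestroyActor sit inside the hit loop, so they run per hit and only when the trace succeeds.
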(event Game|Damage|EventAnyDamage
  (params (Damage :type Float%20%28single-precision%29) (DamageType :type Damage%20Type%20Object%20Reference) (InstigatedBy :type Controller%20Object%20Reference) (DamageCauser :type Actor%20Object%20Reference))
  (bind _returnvalue (Transformation|GetActorLocation))
  (bind _output_get (Variables|Default|SetLife (- (Variables|Default|GetLife) Damage)))
  (if (<= _output_get 0.0)
    (bind (_outhits _returnvalue_2) (Collision|MultiSphereTraceByChannel _returnvalue _returnvalue 2.5e+02 "TraceTypeQuery1" false 0 "ForDuration"))
    (if _returnvalue_2
      (for _array_element _outhits
        (Game|Damage|ApplyDamage (.HitActor (Collision|BreakHitResult _array_element)) 1e+02 0 0)
        (Niagara|SpawnSystematLocation "/Game/FX/NS_Explosion.NS_Explosion" (Transformation|GetActorLocation))
        (Actor|DestroyActor)))))

(fn ConstructionScript)