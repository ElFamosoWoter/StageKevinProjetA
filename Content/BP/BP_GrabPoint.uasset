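; BP_GrabPoint is a grab point that the player can latch onto and jump off from.
; Overlapping its Box shows a prompt widget and starts a timer that polls the player's IsGrab flag.
; On grab, a per-frame timer pins the player to GrabPoint facing the Arrow, with dash, shoot, gravity, wall jump and camera lag disabled.
; Jumping launches the player along the Arrow and upward, then restores those settings.
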(event OnComponentBeginOverlap(Box)
  (params (OverlappedComponent :type Primitive%20Component%20Object%20Reference) (OtherActor :type Actor%20Object%20Reference) (OtherComp :type Primitive%20Component%20Object%20Reference) (OtherBodyIndex :type Integer) (bFromSweep :type Boolean) (SweepResult :type Hit%20Result%20Structure%20%28by%20ref%29))
  (bind _asbp_player (Utilities|Casting|CastToBP_Player OtherActor))
  (Variables|Default|SetAs%20BP%20Player _asbp_player)
  (bind _returnvalue (Utilities|Time|SetTimerbyEvent (delegate Custom|Check) 0.1 true))
  (Variables|Default|SetTimerHANDLE _returnvalue)
  (Development|SetHiddeninGame (Variables|Default|GetWidget) false false))

(event OnComponentEndOverlap(Box)
  (params (OverlappedComponent :type Primitive%20Component%20Object%20Reference) (OtherActor :type Actor%20Object%20Reference) (OtherComp :type Primitive%20Component%20Object%20Reference) (OtherBodyIndex :type Integer))
  (Utilities|Casting|CastToBP_Player OtherActor)
  (Utilities|Time|ClearandInvalidateTimerbyHandle (Variables|Default|GetTimerHANDLE))
  (Development|SetHiddeninGame (Variables|Default|GetWidget) true false))

(event Custom|Check
  (bind _as_bp_player (Variables|Default|GetAs%20BP%20Player))
  (if (Variables|/Game/Player/Blueprints/BP_Player.BP_Player_C|GetIsGrab? (Variables|Default|GetAs%20BP%20Player))
    (Utilities|Time|ClearandInvalidateTimerbyHandle (Variables|Default|GetTimerHANDLE))
    (Variables|/Game/Player/Blueprints/BP_Player.BP_Player_C|SetCanDash? _as_bp_player false)
    (Variables|/Game/Player/Blueprints/BP_Player.BP_Player_C|SetCanShoot? _as_bp_player false)
    (Variables|/Game/Player/Blueprints/BP_Player.BP_Player_C|SetCanGrav? _as_bp_player false)
    (Variables|/Script/Engine.SpringArmComponent|SetbEnableCameraLag (Variables|/Game/Player/Blueprints/BP_Player.BP_Player_C|GetCameraBoom _as_bp_player) false)
    (Variables|/Game/Player/Blueprints/BP_Player.BP_Player_C|SetCanWallJump? _as_bp_player false)
    (bind _returnvalue (Utilities|Time|SetTimerbyEvent (delegate Custom|Grab) 1e-06 true true))
    (Variables|Default|SetNewVar _returnvalue)
    (Development|SetHiddeninGame (Variables|Default|GetWidget) true false)))

(event Custom|Grab
  (bind _arrow (Variables|Default|GetArrow))
  (bind _horif (Variables|Default|GetHoriF))
  (bind _as_bp_player (Variables|Default|GetAs%20BP%20Player))
  (bind _as_bp_player_2 (Variables|Default|GetAs%20BP%20Player))
  (bind _as_bp_player_3 (Variables|Default|GetAs%20BP%20Player))
  (bind _returnvalue (Math|Vector|GetForwardVector _arrow))
  (bind _returnvalue_2 (* _horif _returnvalue))
  (Transformation|SetActorLocation _as_bp_player (Math|Interpolation|VInterpTo (Transformation|GetActorLocation _as_bp_player) (Transformation|GetWorldLocation (Variables|Default|GetGrabPoint)) (Utilities|Time|GetWorldDeltaSeconds) 1e+03) false false)
  (Transformation|SetActorRotation (Variables|Default|GetAs%20BP%20Player) (Transformation|GetWorldRotation (Variables|Default|GetArrow)))
  (if (Variables|/Game/Player/Blueprints/BP_Player.BP_Player_C|GetJump? _as_bp_player_2)
    (Character|LaunchCharacter _as_bp_player_2 (Math|Vector|MakeVector (.x _returnvalue_2) (.y _returnvalue_2) (Variables|Default|GetForce)) false false)
    (Utilities|Time|ClearandInvalidateTimerbyHandle (Variables|Default|GetNewVar))
    (Variables|/Game/Player/Blueprints/BP_Player.BP_Player_C|SetCanDash? _as_bp_player_3 true)
    (Variables|/Game/Player/Blueprints/BP_Player.BP_Player_C|SetCanShoot? _as_bp_player_3 true)
    (Variables|/Game/Player/Blueprints/BP_Player.BP_Player_C|SetCanGrav? _as_bp_player_3 true)
    (Variables|/Script/Engine.SpringArmComponent|SetbEnableCameraLag (Variables|/Game/Player/Blueprints/BP_Player.BP_Player_C|GetCameraBoom _as_bp_player_3) true)
    (Variables|/Game/Player/Blueprints/BP_Player.BP_Player_C|SetCanWallJump? _as_bp_player_3 true)))

(fn ConstructionScript)